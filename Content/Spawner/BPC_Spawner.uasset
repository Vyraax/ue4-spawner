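; Spawner component whose OnSpawn event scatters configured actors inside box areas whose object names match each config entry.
; For each spawn slot it tests actor classes against a random index, with optional random yaw.
; Physics entries spawn at random XY with Z left at zero and simulate physics as BP_Spawnable.
; Others take their height from a downward trace that ignores earlier spawns, using freshly randomized XY.
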(event Custom|OnSpawn
  (params (SpawnAreas :type Array%20of%20Box%20Component%20Object%20References) (Config :type Array%20of%20S%20House%20Areas%20Structures) (Parent :type Actor%20Object%20Reference))
  (for _array_element Config
    (for _array_element_2 SpawnAreas
      (if (Utilities|Enum|Equal(Enum) (Utilities|GetObjectName _array_element_2) (.Name (Utilities|Struct|BreakS_HouseAreas _array_element)))
        (for _index (range 0 (- (.MaxSpawnItems (Utilities|Struct|BreakS_HouseAreas _array_element)) 1))
          (for (_array_element_3 _array_index) (.Actors (Utilities|Struct|BreakS_HouseAreas _array_element))
            (if (== _array_index (Math|Random|RandomIntegerinRange 0 (- (Utilities|Array|Length (.Actors (Utilities|Struct|BreakS_HouseAreas _array_element))) 1)))
              (if (.RandomRotation (Utilities|Struct|BreakS_HouseAreas _array_element))
                (Variables|Default|SetRotationZ (.yaw (Math|Random|RandomRotator false)))
                (else
                  (Variables|Default|SetRotationZ 0.0)))
              (if (.UsePhysics (Utilities|Struct|BreakS_HouseAreas _array_element))
                (bind _returnvalue (Game|SpawnActorfromClass _array_element_3 (Math|Transform|MakeTransform (Math|Vector|MakeVector (.x (Math|Random|RandomPointinBoundingBox (Transformation|GetWorldLocation _array_element_2) (Components|Box|GetScaledBoxExtent _array_element_2))) (.y (Math|Random|RandomPointinBoundingBox (Transformation|GetWorldLocation _array_element_2) (Components|Box|GetScaledBoxExtent _array_element_2))) 0.0) (Math|Rotator|MakeRotator 0.0 0.0 (Variables|Default|GetRotationZ))) "AdjustIfPossibleButAlwaysSpawn" 0 0))
                (bind _asbp_spawnable (Utilities|Casting|CastToBP_Spawnable _returnvalue))
                (Utilities|Array|Add (Variables|Default|GetIgnoreList) _asbp_spawnable)
                (if (Utilities|IsValid _asbp_spawnable)
                  (Physics|SetSimulatePhysics (Variables|/Game/Objects/BP_Spawnable.BP_Spawnable_C|GetStaticMesh _asbp_spawnable) true))
                (else
                  (bind (_outhit _returnvalue_2) (Collision|LineTraceByChannel (Math|Vector|MakeVector (.x (Math|Random|RandomPointinBoundingBox (Transformation|GetWorldLocation _array_element_2) (Components|Box|GetScaledBoxExtent _array_element_2))) (.y (Math|Random|RandomPointinBoundingBox (Transformation|GetWorldLocation _array_element_2) (Components|Box|GetScaledBoxExtent _array_element_2))) (+ (.z (Math|Random|RandomPointinBoundingBox (Transformation|GetWorldLocation _array_element_2) (Components|Box|GetScaledBoxExtent _array_element_2))) 1e+02)) (Math|Vector|MakeVector (.x (Math|Random|RandomPointinBoundingBox (Transformation|GetWorldLocation _array_element_2) (Components|Box|GetScaledBoxExtent _array_element_2))) (.y (Math|Random|RandomPointinBoundingBox (Transformation|GetWorldLocation _array_element_2) (Components|Box|GetScaledBoxExtent _array_element_2))) (- (.z (Math|Random|RandomPointinBoundingBox (Transformation|GetWorldLocation _array_element_2) (Components|Box|GetScaledBoxExtent _array_element_2))) 2e+02)) "TraceTypeQuery1" true (Variables|Default|GetIgnoreList) "None" false "(R=1.000000,G=0.000000,B=0.000000,A=1.000000)" "(R=0.000000,G=1.000000,B=0.000000,A=1.000000)" 15.0))
                  (if (.bblockinghit _outhit)
                    (if _returnvalue_2
                      (if (not (.binitialoverlap _outhit))
                        (bind _returnvalue_3 (Game|SpawnActorfromClass _array_element_3 (Math|Transform|MakeTransform (Math|Vector|MakeVector (.x (Math|Random|RandomPointinBoundingBox (Transformation|GetWorldLocation _array_element_2) (Components|Box|GetScaledBoxExtent _array_element_2))) (.y (Math|Random|RandomPointinBoundingBox (Transformation|GetWorldLocation _array_element_2) (Components|Box|GetScaledBoxExtent _array_element_2))) (.z (.location _outhit))) (Math|Rotator|MakeRotator 0.0 0.0 (Variables|Default|GetRotationZ))) "AdjustIfPossibleButAlwaysSpawn" 0 0))
                        (Utilities|Array|Add (Variables|Default|GetIgnoreList) _returnvalue_3)))))))))))))